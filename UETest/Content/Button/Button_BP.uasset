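; Interactive push button that moves every TurtleBP whose TurtleValue matches its ButtonValue.
; Box overlap with the ThirdPersonCharacter opens and closes a gate on the Interact input, so presses only register nearby.
; A press plays a sound and timelines lerp the button 20 units down and back.
; When that animation finishes, it searches all turtles and calls TurtleMove on matches.
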(event `self.ReceiveBeginPlay`
  (bind (_returnvalue_location _returnvalue_rotation _returnvalue_scale) (`KismetMathLibrary.BreakTransform` (`SceneComponent.GetRelativeTransform` (`self.Button`))))
  (set `self.Out position1` (`KismetMathLibrary.MakeTransform` _returnvalue_location _returnvalue_rotation _returnvalue_scale))
  (set `self.In position1` (`KismetMathLibrary.MakeTransform` (- _returnvalue_location (0.0 0.0 20.0)) _returnvalue_rotation _returnvalue_scale))
  (`self.EnableInput` (`GameplayStatics.GetPlayerController` 0)))

(event `InputAction|Interact`
  (params (Key :type "Key Structure"))
  ;[1 1 1] Button interaction (Push button)
  (:`Pressed`
    (`/Engine/EditorBlueprintResources/StandardMacros.Gate` true :!label _label
      (:`Exit`
        ;[1 1 1] Button animation
        (`GameplayStatics.PlaySoundAtLocation` "/Game/Audio/Button_press.Button_press" (`self.K2_GetActorLocation`) (struct) 1.0 1.0 0.0 null null null)
        (bind (_direction _button_in) (`Timeline|Button In`)
          (:`Update`
            (`SceneComponent.K2_SetRelativeTransform` (`self.Button`) (`KismetMathLibrary.TLerp` (`self.Out position1`) (`self.In position1`) _button_in) false false))
          (:`Finished`
            (bind (_direction_2 _button_in_2) (`Timeline|Button Out` :!via `ReverseFromEnd`)
              (:`Update`
                (`SceneComponent.K2_SetRelativeTransform` (`self.Button`) (`KismetMathLibrary.TLerp` (`self.Out position1`) (`self.In position1`) _button_in_2) false false))
              (:`Finished`
                ;[1 1 1] Button-target
                (bind _outactors (`GameplayStatics.GetAllActorsOfClass` "/Game/Turtle/TurtleBP.TurtleBP_C"))
                (for _array_element _outactors
                  (if (== (`/Game/Turtle/TurtleBP.Turtle value` _array_element) (`self.ButtonValue`))
                    (`/Game/Turtle/TurtleBP.Turtle_move` _array_element null)))))))))))

(event `self.Box.OnComponentBeginOverlap`
  (params (OverlappedComponent :type "PrimitiveComponent Object Reference") (OtherActor :type "Actor Object Reference") (OtherComp :type "PrimitiveComponent Object Reference") (OtherBodyIndex :type Integer) (bFromSweep :type Boolean) (SweepResult :type "HitResult Structure (by ref)"))
  ;[1 1 1] Button interaction (Push button)
  (cast `/Game/ThirdPersonBP/Blueprints/ThirdPersonCharacter` OtherActor)
  (`self.EnableInput` (`GameplayStatics.GetPlayerController` 0))
  (goto _label :!via `Open`))

(event `self.Box.OnComponentEndOverlap`
  (params (OverlappedComponent :type "PrimitiveComponent Object Reference") (OtherActor :type "Actor Object Reference") (OtherComp :type "PrimitiveComponent Object Reference") (OtherBodyIndex :type Integer))
  ;[1 1 1] Button interaction (Push button)
  (cast `/Game/ThirdPersonBP/Blueprints/ThirdPersonCharacter` OtherActor)
  (`self.DisableInput` (`GameplayStatics.GetPlayerController` 0) null)
  (goto _label :!via `Close`))

(fn `UserConstructionScript`)